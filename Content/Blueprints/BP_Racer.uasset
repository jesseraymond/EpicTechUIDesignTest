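; BP_Racer is a skeletal-mesh racer that moves along the BP_Track spline and supplies minimap data.
; BeginPlay finds the track, randomizes speed via ResetRacer and tints the mesh through a dynamic material.
; Each Tick derives spline distance from time since TimeAtLastStart and speed, then sets location and rotation, holding at the spline's end once IsReadyToStart is true.
; Getters expose location, icon with white tint and zero rotation angle.
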(event `self.ReceiveBeginPlay`
  (bind _skeletalmesh (`self.SkeletalMesh`))
  (bind _outactors (`GameplayStatics.GetAllActorsOfClass` "/Game/Blueprints/BP_Track.BP_Track_C"))
  (set `self.Track` (`|GetArrayItem` _outactors))
  (`self.ResetRacer`)
  (bind _returnvalue (`PrimitiveComponent.CreateDynamicMaterialInstance` _skeletalmesh 0 (`|GetArrayItem` (`MeshComponent.GetMaterials` _skeletalmesh)) "None"))
  (`MaterialInstanceDynamic.SetVectorParameterValue` _returnvalue "Tint" (`self.MeshTint`)))

(event `self.ReceiveTick`
  (params (DeltaSeconds :type "Float (single-precision)"))
  (`self.UpdateRacerLocation`))

(fn `GetLocation`
  (returns (Location :type "Vector Structure"))
  (return (`self.K2_GetActorLocation` self)))

(fn `GetMinimapIcon`
  (returns (MinimapIcon :type "Texture2D Object Reference") (Tint :type "LinearColor Structure"))
  (return (`self.MinimapIcon`) (struct :`R` 1.0 :`G` 1.0 :`B` 1.0 :`A` 1.0)))

(fn `GetRotationAngle`
  (returns (RotationAngle :type "Float (double-precision)"))
  (return 0.0))

(fn `ResetRacer`
  (set `self.Speed` (`KismetMathLibrary.RandomFloatInRange` 1.0 1.35)))

(fn `UpdateRacerLocation`
  (bind _track (`self.Track`))
  (bind _spline (`/Game/Blueprints/BP_Track.Spline` _track))
  (bind _returnvalue (`SplineComponent.GetSplineLength` _spline))
  (bind _returnvalue_2 (* (- (`KismetSystemLibrary.GetGameTimeInSeconds`) (`self.TimeAtLastStart`)) (* (`self.Speed`) 1000.0)))
  (if (!= _track null)
    (if (!= _spline null)
      (if (`self.IsReadyToStart`)
        (`self.K2_SetActorLocation` (`SplineComponent.GetLocationAtDistanceAlongSpline` _spline _returnvalue "World"))
        (`self.K2_SetActorRotation` (`SplineComponent.GetRotationAtDistanceAlongSpline` _spline _returnvalue "World"))
        (elif (< _returnvalue_2 (`SplineComponent.GetSplineLength` _spline))
          (bind _output_get (set `self.DistanceAlongSpline` _returnvalue_2))
          (`self.K2_SetActorLocation` (`SplineComponent.GetLocationAtDistanceAlongSpline` _spline _output_get "World"))
          (`self.K2_SetActorRotation` (`SplineComponent.GetRotationAtDistanceAlongSpline` _spline _output_get "World"))
          (else
            (set `self.IsReadyToStart` true)))))))

(fn `UserConstructionScript`)